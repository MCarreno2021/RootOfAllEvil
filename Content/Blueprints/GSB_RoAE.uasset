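; GSB_RoAE, likely a game state Blueprint, scales a difficulty multiplier with elapsed game time.
; Each Tick, it truncates game time to whole minutes and stores that as DifficultyMultiplier, with a minimum of 1, so the first increase comes at two minutes.
; It prints both the minute count and the multiplier on screen every frame as debug output.
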(event `self.ReceiveBeginPlay`)

(event `self.ReceiveTick`
  (params (DeltaSeconds :type "Float (single-precision)"))
  (bind _returnvalue (`KismetMathLibrary.FTrunc` (/ (`KismetSystemLibrary.GetGameTimeInSeconds`) 60.0)))
  (`KismetSystemLibrary.PrintString` (`KismetStringLibrary.Conv_IntToString` _returnvalue) true true (struct :`R` 1.0 :`G` 0.922295 :`B` 0.095428 :`A` 1.0) 0.1)
  (if (< _returnvalue 1)
    (bind _output_get (set `self.DifficultyMultiplier` (+ _returnvalue 1)))
    (else
      (set `self.DifficultyMultiplier` _returnvalue)))
  (`KismetSystemLibrary.PrintString` (`KismetStringLibrary.Conv_IntToString` _output_get) true true (struct :`G` 0.66 :`B` 1.0 :`A` 1.0) 0.1))

(fn `UserConstructionScript`)
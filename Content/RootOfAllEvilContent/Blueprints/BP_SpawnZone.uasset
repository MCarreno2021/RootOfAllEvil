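; BP_SpawnZone periodically spawns random enemies inside a box until the world-wide AI_Enemy_Base count reaches EnemyAmount.
; A self-recalling SpawnCheck loop, started on BeginPlay, picks a random point and yaw, then line-traces down to place each spawn above the ground.
; Spawning pauses while BP_FirstPersonCharacter overlaps FallOffZone and resumes on exit.
; The construction script applies configurable sizes to both boxes and positions FallOffZone.
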(event `SpawnCheck`
  (bind _spawnzone (`self.SpawnZone`))
  (if (`self.Active?`) :!label _label
    (bind _outactors (`GameplayStatics.GetAllActorsOfClass` "/Game/FirstPerson/Blueprints/AI_Enemy_Base.AI_Enemy_Base_C"))
    (if (not (>= (`KismetArrayLibrary.Array_Length` _outactors) (`self.EnemyAmount`)))
      (bind _returnvalue (`|SpawnActorFromClass` (`KismetArrayLibrary.Array_Random` (`self.EnemysToSpawn`)) (`KismetMathLibrary.MakeTransform` (`KismetMathLibrary.RandomPointInBoundingBox` (`SceneComponent.K2_GetComponentLocation` _spawnzone) (`BoxComponent.GetScaledBoxExtent` _spawnzone)) (`KismetMathLibrary.MakeRotator` 0.0 0.0 (`KismetMathLibrary.RandomFloatInRange` -180.0 180.0))) "Undefined" "OverrideRootScale" null null))
      (`/Engine/EditorBlueprintResources/StandardMacros.IsValid` _returnvalue
        (:`Is Valid`
          (bind _output_get (set `self.SpawnedUnit` _returnvalue))
          (bind _returnvalue_2 (`self.K2_GetActorLocation` _returnvalue))
          (bind (_outhit _returnvalue_3) (`KismetSystemLibrary.LineTraceSingle` _returnvalue_2 (- _returnvalue_2 (0.0 0.0 1000.0)) "TraceTypeQuery1" false (`|MakeArray` _output_get :!type "Actor Object Reference") "ForOneFrame"))
          (if _returnvalue_3
            (`self.K2_SetActorLocation` (`self.SpawnedUnit`) (+ (`.Location` (`GameplayStatics.BreakHitResult` _outhit)) (0.0 0.0 90.0)) false false)))
        (:`Is Not Valid`
          _))))
  (`KismetSystemLibrary.Delay` (`self.SpawnDelay`))
  (`self.SpawnCheck`))

(event `self.ReceiveBeginPlay`
  (goto _label))

(event `self.FallOffZone.OnComponentBeginOverlap`
  (params (OverlappedComponent :type "PrimitiveComponent Object Reference") (OtherActor :type "Actor Object Reference") (OtherComp :type "PrimitiveComponent Object Reference") (OtherBodyIndex :type Integer) (bFromSweep :type Boolean) (SweepResult :type "HitResult Structure (by ref)"))
  (cast `/Game/FirstPerson/Blueprints/BP_FirstPersonCharacter` OtherActor)
  (set `self.Active?` false)
  (`KismetSystemLibrary.PrintString` "Deactivated Spawn"))

(event `self.FallOffZone.OnComponentEndOverlap`
  (params (OverlappedComponent :type "PrimitiveComponent Object Reference") (OtherActor :type "Actor Object Reference") (OtherComp :type "PrimitiveComponent Object Reference") (OtherBodyIndex :type Integer))
  (cast `/Game/FirstPerson/Blueprints/BP_FirstPersonCharacter` OtherActor)
  (set `self.Active?` true)
  (`KismetSystemLibrary.PrintString` "Activated Spawn"))

(fn `UserConstructionScript`
  (bind _falloffzone (`self.FallOffZone`))
  (`BoxComponent.SetBoxExtent` (`self.SpawnZone`) (`self.SpawnZoneSize`) true)
  (`BoxComponent.SetBoxExtent` _falloffzone (`self.FallOffZoneSize`) true)
  (`SceneComponent.K2_SetRelativeLocation` _falloffzone (`self.FallOfZoneLocation`) false false))
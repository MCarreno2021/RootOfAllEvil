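; GSB_RoAE is a Blueprint, apparently the game state for RootOfAllEvil, that scales a DifficultyMultiplier with elapsed play time.
; Every Tick it sets the multiplier to the whole minutes of game time, with a floor of one, so it first rises at the two-minute mark.
; BeginPlay and the construction script are empty, and the debug print nodes are disconnected.
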(event `self.ReceiveBeginPlay`)

(event `self.ReceiveTick`
  (params (DeltaSeconds :type "Float (single-precision)"))
  (bind _returnvalue (`KismetMathLibrary.FTrunc` (/ (`KismetSystemLibrary.GetGameTimeInSeconds`) 60.0)))
  (if (< _returnvalue 1)
    (bind _output_get (set `self.DifficultyMultiplier` (+ _returnvalue 1)))
    (else
      (set `self.DifficultyMultiplier` _returnvalue))))

(fn `UserConstructionScript`)
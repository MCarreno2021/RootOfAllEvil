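; BP_Temp is an actor that handles the main menu and game pausing.
; BeginPlay pauses the game and shows WBP_MainMenu, sharing the open branch of the IA_Menu toggle.
; Opening creates the widget once, reuses it afterwards, and switches to focused UI-only input with a visible, locked cursor.
; When IA_Menu triggers while paused, it unpauses, removes the widget, hides the cursor and restores game-only input.
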(event `EnhancedInput|/Game/FirstPerson/Input/Actions/IA_Menu`
  (params (ActionValue :type Boolean) (ElapsedSeconds :type "Float (double-precision)") (TriggeredSeconds :type "Float (double-precision)") (InputAction :type "InputAction Object Reference" :default "/Game/FirstPerson/Input/Actions/IA_Menu.IA_Menu"))
  (bind _returnvalue (`GameplayStatics.GetPlayerController` 0))
  (bind _returnvalue_2 (`GameplayStatics.GetPlayerController` 0))
  (bind _wbp_mainmenu (`self.WBP_MainMenu`))
  (:`Triggered`
    (if (`GameplayStatics.IsGamePaused`)
      (`GameplayStatics.SetGamePaused` false)
      (`WidgetBlueprintLibrary.SetInputMode_GameOnly` _returnvalue_2)
      (`Widget.RemoveFromParent` (`self.WBP_MainMenu`))
      (set `PlayerController.bShowMouseCursor` false _returnvalue_2)
      (else
        (`GameplayStatics.SetGamePaused` true :!label _label)
        (`/Engine/EditorBlueprintResources/StandardMacros.IsValid` (`self.WBP_MainMenu`)
          (:`Is Valid`
            _)
          (:`Is Not Valid`
            (bind _returnvalue_3 (`|CreateWidget` "/Game/RootOfAllEvilContent/Blueprints/WBP_MainMenu.WBP_MainMenu_C"))
            (set `self.WBP_MainMenu` _returnvalue_3)))
        (`UserWidget.AddToViewport` (`self.WBP_MainMenu`) 0)
        (set `PlayerController.bShowMouseCursor` true _returnvalue)
        (`Widget.SetKeyboardFocus` _wbp_mainmenu)
        (`WidgetBlueprintLibrary.SetInputMode_UIOnlyEx` _returnvalue _wbp_mainmenu "LockAlways" true)))))

(event `self.ReceiveBeginPlay`
  (goto _label))

(fn `UserConstructionScript`)